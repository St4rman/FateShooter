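; BP_Launcher is a launcher weapon Blueprint that equips itself to the character who picks it up.
; Its PickupComponent's OnPickUp event calls AttachWeapon and, on success, sets the rifle flag and weapon animation type on the first-person AnimBP.
; It then flags BP_FateCharacter as armed, updates the HUD crosshair, and registers itself as the current weapon with that character as owner.
; The graph contains no firing logic.
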(event OnPickUp(PickupComponent)
  (params (PickUpCharacter :type Project%20Fate%20Character%20Object%20Reference))
  ;[0 0 0 0.5 44] Equip Code
  (bind _returnvalue (Class|FateWeaponBase|AttachWeapon PickUpCharacter))
  (if _returnvalue
    (bind _asfirst_person_anim_bp (Utilities|Casting|CastToFirstPerson_AnimBP (Components|SkeletalMesh|GetAnimInstance (Variables|/Script/ProjectFate.ProjectFateCharacter|GetMesh1P PickUpCharacter))))
    (Variables|/Game/FirstPersonArms/Animations/FirstPerson_AnimBP.FirstPerson_AnimBP_C|SetHasRifle _asfirst_person_anim_bp true)
    (Variables|/Game/FirstPersonArms/Animations/FirstPerson_AnimBP.FirstPerson_AnimBP_C|SetWeaponAnimType _asfirst_person_anim_bp (Variables|Default|GetWeaponAnimType))
    (bind _asbp_fate_character (Utilities|Casting|CastToBP_FateCharacter PickUpCharacter))
    (Variables|/Game/MyBlueprints/Player/BP_FateCharacter.BP_FateCharacter_C|SetHasWeapon _asbp_fate_character true)
    (Default|UpdateWeaponCrosshairs (Variables|/Game/MyBlueprints/Player/BP_FateCharacter.BP_FateCharacter_C|GetPlayerHUD _asbp_fate_character) (Variables|Default|GetCrossHairTexture))
    (Variables|/Script/ProjectFate.ProjectFateCharacter|SetCurrentWeapon PickUpCharacter self)
    (Actor|SetOwner PickUpCharacter)))

(fn ConstructionScript)