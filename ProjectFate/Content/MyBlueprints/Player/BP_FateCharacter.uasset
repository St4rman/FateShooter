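; BP_FateCharacter is the player character Blueprint, handling local UI, strafe camera lean and death.
; BeginPlay or SetUpUI creates the HUD and health bar widgets.
; Each tick, DoLeanMacro interpolates control rotation roll toward a lean angle signed by horizontal move input, or back to zero.
; On death, it sends a kill message to the gameplay game mode, clears weapons via ServerClearWeapons and requests respawn through the player controller.
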(event Custom|SetUpUI
  (bind _returnvalue (Class|GameplayStatics|GetPlayerControllerfromID))
  (bind _returnvalue_2 (UserInterface|CreateWidget "/Game/MyContent/UI/Game/WBP_HUD.WBP_HUD_C" _returnvalue))
  (Variables|Default|SetPlayerHUD _returnvalue_2)
  (UserInterface|Viewport|AddtoViewport _returnvalue_2 0)
  (bind _returnvalue_3 (UserInterface|CreateWidget "/Game/MyContent/UI/Game/WBP_HealthBar.WBP_HealthBar_C" _returnvalue))
  (Variables|Default|SetHealthBar _returnvalue_3)
  (UserInterface|Viewport|AddtoViewport _returnvalue_3 0))

(event EventBeginPlay
  (bind _returnvalue (Class|GameplayStatics|GetPlayerControllerfromID))
  (bind _returnvalue_2 (UserInterface|CreateWidget "/Game/MyContent/UI/Game/WBP_HUD.WBP_HUD_C" _returnvalue))
  (Variables|Default|SetPlayerHUD _returnvalue_2)
  (UserInterface|Viewport|AddtoViewport _returnvalue_2 0)
  (bind _returnvalue_3 (UserInterface|CreateWidget "/Game/MyContent/UI/Game/WBP_HealthBar.WBP_HealthBar_C" _returnvalue))
  (Variables|Default|SetHealthBar _returnvalue_3)
  (UserInterface|Viewport|AddtoViewport _returnvalue_3 0))

(event EventDoCamLean
  (bind _camleanspeed (Variables|Default|GetCamLeanSpeed))
  ;[0 0 0 0.5] Cam lean
  (bind _returnvalue (Class|ProjectFateCharacter|ShouldCamLean))
  (if _returnvalue
    (Math|Float|CompareFloat (.x (Input|EnhancedActionValues|GetIA_Move)) 0.0
      (:>
        (Utilities|DoLeanMacro (Variables|Default|GetCamLeanAngle) _camleanspeed))
      (:<
        (Utilities|DoLeanMacro (* (Variables|Default|GetCamLeanAngle) -1.0) _camleanspeed)))
    (else
      (Utilities|DoLeanMacro 0.0 _camleanspeed))))

(event EventTick
  (params (DeltaSeconds :type Float%20%28single-precision%29))
  ;[0 0 0 0.5] Cam lean
  (Class|ProjectFateCharacter|DoCamLean))

(event EventOnPlayerDeath
  (params (InstigatorPlayer :type Player%20State%20Object%20Reference))
  (bind _asbp_gm_gameplay (Utilities|Casting|CastToBP_GM_Gameplay (Game|GetGameMode)))
  (Class|BPIGameMode|NotifyonPlayerKill(Message) _asbp_gm_gameplay InstigatorPlayer (Variables|Default|GetPlayerState self))
  (bind _asbp_pc_gameplay (Utilities|Casting|CastToBP_PC_Gameplay (Pawn|GetController)))
  (Class|ProjectFateCharacter|ServerClearWeapons)
  (Default|SRRespawn _asbp_pc_gameplay))

(fn ConstructionScript)