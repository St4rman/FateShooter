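; Gameplay GameState that starts a match countdown once enough players have connected.
; A player-connect notification updates the player count and, on reaching the minimum, sets the replicated countdown a single time.
; Its RepNotify refreshes every countdown widget and, on authority, drives a self-retriggering one-second decrement loop, flagging the match as started at zero.
; A separate reset event zeroes the countdown directly.
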(event Custom|MatchCountdown
  (Utilities|FlowControl|Delay 1.0)
  (Variables|Default|SetMatchStartCountdown (- (Variables|Default|GetMatchStartCountdown) 1)))

(event Custom|ResetTimer
  (Variables|Default|SetMatchStartCountdown 0))

(event EventBeginPlay)

(event EventTick
  (params (DeltaSeconds :type Float%20%28single-precision%29)))

(event EventNotifyonPlayerConnect
  (bind _returnvalue (Class|GameplayStatics|GetNumPlayerStates))
  (Variables|Default|SetCurrentPlayerCount _returnvalue)
  (if (>= _returnvalue (Variables|Default|GetMinimumPlayerCount))
    (Utilities|FlowControl|DoOnce false
      (:Completed
        (Variables|Default|SetMatchStartCountdown 10)))))

(fn ConstructionScript
  (|CallParentFunction))

(fn OnRepMatchStartCountdown
  (CallFunction|UpdateMatchCountdownWidget)
  (Networking|SwitchHasAuthority
    (:Authority
      (if (== (Variables|Default|GetMatchStartCountdown) 10)
        (CallFunction|MatchCountdown)
        (elif (== (Variables|Default|GetMatchStartCountdown) 0)
          (Variables|Default|SetHasStarted true)
          (else
            (CallFunction|MatchCountdown)))))))

(fn UpdateMatchCountdownWidget
  (bind _foundwidgets (Widget|GetAllWidgetsOfClass "/Game/MyContent/UI/Game/WBP_MatchStartCountdown.WBP_MatchStartCountdown_C" false))
  (for _array_element _foundwidgets
    (Default|UpdateCountdown _array_element (Variables|Default|GetMatchStartCountdown))))