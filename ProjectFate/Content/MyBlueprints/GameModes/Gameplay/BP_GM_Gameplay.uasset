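; Gameplay Game Mode that tracks player controllers, spawns players and handles kill scoring and kill-feed updates.
; Login and logout update the controller list and notify the GameState.
; SpawnPlayer replaces the controlled pawn with a BP_FateCharacter at a random PlayerStart and sets up health UI.
; Kills update the instigator's PlayerState score and set the RepNotify KillFeed, though the Steam persona-name lookups meant to fill it are disconnected.
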(event Custom|NotifySpawnUI
  (params (Instigator :type Player%20State%20Object%20Reference) (Target :type Player%20State%20Object%20Reference))
  (Utilities|FlowControl|Sequence
    (:then_2
      (Variables|Default|SetKillFeed (Variables|Default|GetLocalKillFeed)))))

(event EventBeginPlay
  (|CallParentFunction) ; This node is disabled and will not be called.\nDrag off pins to build functionality.
)

(event EventTick
  (params (DeltaSeconds :type Float%20%28single-precision%29))
  (|CallParentFunction DeltaSeconds) ; This node is disabled and will not be called.\nDrag off pins to build functionality.
)

(event EventPostLogin
  (params (NewPlayer :type Player%20Controller%20Object%20Reference))
  (bind _asbp_pc_gameplay (Utilities|Casting|CastToBP_PC_Gameplay NewPlayer))
  (Utilities|Array|AddUnique (Variables|Default|GetPlayerControllers) _asbp_pc_gameplay)
  (Class|BPIGameState|NotifyonPlayerConnect(Message) (Game|GetGameState)))

(event EventOnLogout
  (params (ExitingController :type Controller%20Object%20Reference))
  (bind _asbp_pc_gameplay (Utilities|Casting|CastToBP_PC_Gameplay ExitingController))
  (Utilities|Array|RemoveItem (Variables|Default|GetPlayerControllers) _asbp_pc_gameplay)
  (Class|BPIGameState|NotifyonPlayerConnect(Message) (Game|GetGameState)))

(event EventNotifyonPlayerKill
  (params (Instigator :type Player%20State%20Object%20Reference) (DeadPlayer :type Player%20State%20Object%20Reference))
  (bind _asbp_ps_gameplay (Utilities|Casting|CastToBP_PS_Gameplay Instigator))
  (Default|UpdateScore _asbp_ps_gameplay)
  (CallFunction|NotifySpawnUI Instigator DeadPlayer))

(fn ConstructionScript
  (|CallParentFunction))

(fn FindPlayerStartLoc
  (bind _outactors (Actor|GetAllActorsOfClass "/Script/Engine.PlayerStart"))
  (return (Transformation|GetActorTransform (Utilities|Array|Get(acopy) _outactors (Math|Random|RandomIntegerinRange 0 (- (Utilities|Array|Length _outactors) 1))))))

(fn SpawnPlayer
  (params (PlayerController :type Player%20Controller%20Object%20Reference))
  (bind _returnvalue (Pawn|GetControlledPawn PlayerController))
  (Utilities|IsValid _returnvalue
    (:Is%20Valid
      (Actor|DestroyActor _returnvalue))
    (:Is%20Not%20Valid
      _))
  (bind _returnvalue_2 (Game|SpawnActorfromClass "/Game/MyBlueprints/Player/BP_FateCharacter.BP_FateCharacter_C" (Spawn|FindPlayerStartLoc) "Undefined" "MultiplyWithRoot" 0 3.0 0))
  (Pawn|Possess PlayerController _returnvalue_2)
  (Default|SetupHealthUI _returnvalue_2))

(fn UpdateGMPlayerList)

(fn OnRepPlayerControllers)

(fn OnRepKillFeed
  (bind _killfeed (Variables|Default|GetKillFeed))
  (CallFunction|AddKillNotify (Utilities|Text|ToText(String) (Utilities|Array|Get(acopy) _killfeed)) (Utilities|Text|ToText(String) (Utilities|Array|Get(acopy) _killfeed))))