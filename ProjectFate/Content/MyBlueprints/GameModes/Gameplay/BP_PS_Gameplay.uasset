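; Gameplay PlayerState that tracks each player's kill count against the match's score to beat.
; On BeginPlay it caches the target score from BP_GS_Gameplay.
; UpdateScore increments the count and, when it exactly equals the target, calls OnServ on the player's BP_FateCharacter pawn.
; ResetScore sets the count back to zero.
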(event Custom|UpdateScore
  (bind _output_get (Variables|Default|SetPlayerKillCount (+ (Variables|Default|GetPlayerKillCount) 1)))
  (if (== _output_get (Variables|Default|GetScoretobeat))
    (bind _asbp_fate_character (Utilities|Casting|CastToBP_FateCharacter (PlayerState|GetPawn)))
    (Default|OnServ _asbp_fate_character)))

(event Custom|ResetScore
  (Variables|Default|SetPlayerKillCount 0))

(event EventBeginPlay
  (bind _asbp_gs_gameplay (Utilities|Casting|CastToBP_GS_Gameplay (Game|GetGameState)))
  (Variables|Default|SetScoretobeat (Variables|/Game/MyBlueprints/GameModes/Gameplay/BP_GS_Gameplay.BP_GS_Gameplay_C|GetScoreToBeat _asbp_gs_gameplay)))

(fn ConstructionScript)